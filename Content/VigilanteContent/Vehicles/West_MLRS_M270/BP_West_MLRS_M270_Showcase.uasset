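; Showcase variant of the West M270 MLRS vehicle Blueprint that exposes its adjustable features to showcase UI controls.
; Indexed slider events forward values to setters for wheel speed, launcher elevation and rotation, doors, hatches and light emissivity.
; A checkbox event toggles the damaged look and a button event selects the skin type, converting the index to a double.
; The construction script only calls the parent's.
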(event `/Game/VigilanteContent/Shared/Blueprints/Showcase/Interfaces/BP_ShowcaseControlsInterface.SetSliderVariable0`
  (params (NewValue :type "Float (double-precision)"))
  ;[1 1 1] Showcase float controls
  (`self.SetWheelSpeed` NewValue))

(event `/Game/VigilanteContent/Shared/Blueprints/Showcase/Interfaces/BP_ShowcaseControlsInterface.SetCheckboxVariable0`
  (params (NewState :type Boolean))
  ;[1 1 1] Showcase checkbox controls
  (`self.SetShowDamaged` NewState))

(event `/Game/VigilanteContent/Shared/Blueprints/Showcase/Interfaces/BP_ShowcaseControlsInterface.SetButtonsVariable0`
  (params (NewIndex :type Integer))
  ;[1 1 1] Showcase button controls
  (`self.SetSkinType` (`KismetMathLibrary.Conv_IntToDouble` NewIndex)))

(event `/Game/VigilanteContent/Shared/Blueprints/Showcase/Interfaces/BP_ShowcaseControlsInterface.SetSliderVariable1`
  (params (NewValue :type "Float (double-precision)"))
  ;[1 1 1] Showcase float controls
  (`self.SetRocketLauncherElevation` NewValue))

(event `/Game/VigilanteContent/Shared/Blueprints/Showcase/Interfaces/BP_ShowcaseControlsInterface.SetSliderVariable2`
  (params (NewValue :type "Float (double-precision)"))
  ;[1 1 1] Showcase float controls
  (`self.SetRocketLauncherRotation` NewValue))

(event `/Game/VigilanteContent/Shared/Blueprints/Showcase/Interfaces/BP_ShowcaseControlsInterface.SetSliderVariable3`
  (params (NewValue :type "Float (double-precision)"))
  ;[1 1 1] Showcase float controls
  (`self.SetDoors` NewValue))

(event `/Game/VigilanteContent/Shared/Blueprints/Showcase/Interfaces/BP_ShowcaseControlsInterface.SetSliderVariable4`
  (params (NewValue :type "Float (double-precision)"))
  ;[1 1 1] Showcase float controls
  (`self.SetDoorHatches` NewValue))

(event `/Game/VigilanteContent/Shared/Blueprints/Showcase/Interfaces/BP_ShowcaseControlsInterface.SetSliderVariable5`
  (params (NewValue :type "Float (double-precision)"))
  ;[1 1 1] Showcase float controls
  (`self.SetFrontHatches` NewValue))

(event `/Game/VigilanteContent/Shared/Blueprints/Showcase/Interfaces/BP_ShowcaseControlsInterface.SetSliderVariable6`
  (params (NewValue :type "Float (double-precision)"))
  ;[1 1 1] Showcase float controls
  (`self.SetRoofHatch` NewValue))

(event `/Game/VigilanteContent/Shared/Blueprints/Showcase/Interfaces/BP_ShowcaseControlsInterface.SetSliderVariable7`
  (params (NewValue :type "Float (double-precision)"))
  ;[1 1 1] Showcase float controls
  (`self.SetLightsEmissivity` NewValue))

(fn `UserConstructionScript`
  (`parent.UserConstructionScript`))